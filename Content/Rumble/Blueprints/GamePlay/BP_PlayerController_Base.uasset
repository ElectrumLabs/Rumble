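; Base player controller for Rumble that manages a player's spawning, respawning, UI, disconnects and weapon input.
; After login the client builds the HUD and in-game menu, then sends its lobby-selected class to the server, which possesses it at an unused spawn point.
; Class and spawn point are cached for respawns.
; Input toggles scoreboard and menu, and fires pistol bullets from player 0's pawn through a timer-reopened gate.
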(event Custom|UpdateScoreboard
  ;[0 1 0] Client | Just an event to manualy update the PlayerList in the Scoreboard
  (Utilities|IsValid (Variables|WidgetReference|GetScoreboardWidgetRef)
    (:Is%20Valid
      (Default|RefreshPlayerList (Variables|WidgetReference|GetScoreboardWidgetRef))
      (Default|AddWidgetsasChild (Variables|WidgetReference|GetScoreboardWidgetRef)))))

(event Custom|ClientDisconnect
  (params (bInDisplayReason :type Boolean) (InReason :type Text))
  ;[0 1 0] Client | Disconncets the Client with a specific reason. Also used for kicking a player. Sends him back to the MainMenu
  (Utilities|IsValid (Variables|References|GetGameInstanceRef)
    (:Is%20Valid
      _)
    (:Is%20Not%20Valid
      (CallFunction|SetupReferences)))
  (if bInDisplayReason
    (Utilities|Array|Add (Variables|/Game/Rumble/Blueprints/BlueprintsUsedInAllMaps/BP_GameInstance.BP_GameInstance_C|GetPendingErrorMessage (Variables|References|GetGameInstanceRef)) InReason))
  (Development|ExecuteConsoleCommand "Disconnect" self)
  (Default|TransitiontoMainMenu (Variables|References|GetGameInstanceRef)))

(event Custom|SetupReferences
  (bind _returnvalue (Game|GetGameState))
  (bind _returnvalue_2 (Game|GetGameInstance))
  (bind _playerstate (Variables|GetPlayerState))
  ;[1 1 1] Save all kinds of important reference, so we don't have to cast all the time
  (Utilities|FlowControl|Sequence
    (:then_0
      (Utilities|IsValid _returnvalue_2
        (:Is%20Valid
          (bind _asbp_game_instance (Utilities|Casting|CastToBP_GameInstance _returnvalue_2))
          (Variables|References|SetGameInstanceRef _asbp_game_instance))))
    (:then_1
      (Utilities|IsValid _returnvalue
        (:Is%20Valid
          (bind _asbp_game_state_base (Utilities|Casting|CastToBP_GameState_Base _returnvalue))
          (Variables|References|SetGameStateRef _asbp_game_state_base))))
    (:then_2
      (Utilities|IsValid _playerstate
        (:Is%20Valid
          (bind _asbp_player_state_base (Utilities|Casting|CastToBP_PlayerState_Base _playerstate))
          (Variables|References|SetPlayerStateRef _asbp_player_state_base))))))

(event Custom|ServerSpawnMe
  (params (InCharacterClass :type BP%20Character%20Base%20Class%20Reference))
  ;[1 0 0] Clients and Server | This handles the initial spawn of the Players
  (Variables|SpawnSystem|SetClassToReSpawn InCharacterClass)
  (CallFunction|HandleSpawningPlayer))

(event Custom|ServerRestartGame
  (bind _gamestateref (Variables|References|GetGameStateRef))
  ;[1 0 1] Server | Resets our Game
  (Utilities|IsValid _gamestateref
    (:Is%20Valid
      (Default|ResetGame _gamestateref))))

(event Custom|ClientPostLogin
  (bind _gameinstanceref (Variables|References|GetGameInstanceRef))
  ;[1 0 0] Clients and Server | This handles the initial spawn of the Players
  ;;[1 1 0] Client | Creates the UI and asks the Server to spawn the Player providing a class from the lobby selection
  (CallFunction|SetupGameUI)
  (Utilities|IsValid _gameinstanceref
    (:Is%20Valid
      _)
    (:Is%20Not%20Valid
      (CallFunction|SetupReferences)))
  (CallFunction|ServerSpawnMe (.class (Variables|/Game/Rumble/Blueprints/BlueprintsUsedInAllMaps/BP_GameInstance.BP_GameInstance_C|GetSelectedCharacterClass _gameinstanceref))))

(event Custom|RespawnPlayer
  (bind _returnvalue (Pawn|GetControlledPawn))
  (bind _spawnpoint (Variables|SpawnSystem|GetSpawnPoint))
  ;[1 0 0] This handles our Respawn
  ;;[1 1 0] Server | We try to respawn the Player at the already known SpawnPoint, with the already known Class and possess it again
  (Utilities|IsValid _returnvalue
    (:Is%20Valid
      (Actor|DestroyActor _returnvalue))
    (:Is%20Not%20Valid
      _))
  (Utilities|IsValid _spawnpoint
    (:Is%20Valid
      (bind _returnvalue_2 (Game|SpawnActorfromClass (Variables|SpawnSystem|GetClassToReSpawn) (Math|Transform|MakeTransform (Transformation|GetWorldLocation _spawnpoint) (Transformation|GetWorldRotation _spawnpoint) "1,1,1") "AlwaysSpawn" 0 0))
      (Utilities|IsValid _returnvalue_2
        (:Is%20Valid
          (Pawn|Possess _returnvalue_2)
          (Default|ResetHealthandWeapon (Variables|References|GetPlayerStateRef)))))))

(event EventBeginPlay
  (bind _playerstate (Variables|GetPlayerState))
  (CallFunction|SetupReferences)
  ;[1 0 0] Server | Keep track of begin the Server, so we can use this in our widgets
  (if (and (Networking|IsServer) (Pawn|IsLocalPlayerController))
    (Utilities|IsValid _playerstate
      (:Is%20Valid
        (bind _asbp_player_state_base (Utilities|Casting|CastToBP_PlayerState_Base _playerstate))
        (Variables|/Game/Rumble/Blueprints/GamePlay/BP_PlayerState_Base.BP_PlayerState_Base_C|SetIsServer _asbp_player_state_base true)))))

(event Input|ActionEvents|InputActionMenu
  (params (Key :type Key%20Structure))
  ;[1 0 0] This handles displaying and removing widgets that are important while playing. Driven by Key Inputs
  ;;[0 0 0] Open our ingame menu
  (:Pressed
    (if (Variables|WidgetSystem|GetbIngameMenuOpen)
      (Widget|RemovefromParent (Variables|WidgetReference|GetInGameMenuWidgetRef))
      (Input|SetInputModeGameOnly self)
      (Variables|WidgetSystem|SetbIngameMenuOpen false)
      (Variables|Default|SetbShowMouseCursor false)
      (else
        (UserInterface|Viewport|AddtoViewport (Variables|WidgetReference|GetInGameMenuWidgetRef) 0)
        (Input|SetInputModeUIOnly self (Variables|WidgetReference|GetInGameMenuWidgetRef) "DoNotLock")
        (Variables|WidgetSystem|SetbIngameMenuOpen true)
        (Variables|Default|SetbShowMouseCursor true)))))

(event Input|ActionEvents|InputActionScoreboard
  (params (Key :type Key%20Structure))
  ;[1 0 0] This handles displaying and removing widgets that are important while playing. Driven by Key Inputs
  ;;[0 0 0] TAB press and release handles the display of the Scoreboard
  (:Pressed
    (Utilities|IsValid (Variables|WidgetReference|GetScoreboardWidgetRef)
      (:Is%20Valid
        (UserInterface|Viewport|AddtoViewport (Variables|WidgetReference|GetScoreboardWidgetRef) 0)
        (Variables|WidgetSystem|SetbScoreboardOpen true))))
  (:Released
    (Utilities|IsValid (Variables|WidgetReference|GetScoreboardWidgetRef)
      (:Is%20Valid
        (Widget|RemovefromParent (Variables|WidgetReference|GetScoreboardWidgetRef))
        (Variables|WidgetSystem|SetbScoreboardOpen false)))))

(event Input|ActionEvents|InputActionFireWeapon
  (params (Key :type Key%20Structure))
  ;[1 1 1] Fire the current weapon equipped
  (:Pressed
    (if (Variables|/Game/Rumble/Blueprints/GamePlay/BP_PlayerState_Base.BP_PlayerState_Base_C|GetbCanShoot (Variables|References|GetPlayerStateRef))
      (Variables|Player|SetbLeftMouseDown true)
      (switch Utilities|FlowControl|Switch|SwitchonEWeaponsList (Variables|/Game/Rumble/Blueprints/GamePlay/BP_PlayerState_Base.BP_PlayerState_Base_C|GetMyWeapons (Variables|References|GetPlayerStateRef))
        (:NewEnumerator0
          (CallFunction|BasicPistolFire)))))
  (:Released
    (Variables|Player|SetbLeftMouseDown false)))

(event Custom|BasicPistolFire
  (bind (_rotation _location) (CallFunction|FireatLocation 0.0 0.0))
  (bind _returnvalue (Game|GetPlayerCharacter 0))
  (Utilities|FlowControl|Gate false
    (:Exit
      (Game|SpawnActorfromClass "/Game/Rumble/Weapons/BP_Bullet.BP_Bullet_C" (Math|Transform|MakeTransform _location _rotation "1,1,1") "AlwaysSpawn" _returnvalue _returnvalue)
      (bind _returnvalue_2 (Utilities|Time|SetTimerbyEvent (delegate Custom|PistolOpen) 2.0))
      (Variables|WeaponTimers|SetPistolTimer _returnvalue_2))))

(event Custom|PistolOpen
  (bind (_rotation _location) (CallFunction|FireatLocation 0.0 0.0))
  (bind _returnvalue (Game|GetPlayerCharacter 0))
  (Utilities|FlowControl|Gate false) ; enters at Open
)

(event Custom|PistolClose
  (bind (_rotation _location) (CallFunction|FireatLocation 0.0 0.0))
  (bind _returnvalue (Game|GetPlayerCharacter 0))
  (Utilities|FlowControl|Gate false) ; enters at Close
)

(fn ConstructionScript)

(fn SetupGameUI
  ;[1 1 1] Creating our MainHUDWidget for all PlayerControllers, since this is the same in all of them
  (if (Pawn|IsLocalPlayerController)
    (bind _returnvalue (UserInterface|CreateWidget "/Game/Rumble/Widgets/GamePlayBaseWidgets/HUDWidgets/W_MainHUDWidget.W_MainHUDWidget_C" self))
    (bind _output_get (Variables|WidgetReference|SetHUDWidgetRef _returnvalue))
    (UserInterface|Viewport|AddtoViewport _output_get 0)
    ;[1 1 1] Also creating our IngameMenu. All of our GameModes have this
    (bind _returnvalue_2 (UserInterface|CreateWidget "/Game/Rumble/Widgets/GamePlayBaseWidgets/IngameMenuWidgets/W_InGameMenu.W_InGameMenu_C" self (Variables|WidgetSystem|GetPlayerListEntryClass)))
    (Variables|WidgetReference|SetInGameMenuWidgetRef _returnvalue_2)))

(fn HandleSpawningPlayer
  ;[1 1 0] Server | Spawns the Player with the given "Class" and saves the SpawnPoint as well as the class so we can respawn him easier later. We make sure that the we use a SpawnPoint that is not already taken
  (bind _outactors (Actor|GetAllActorsOfClass "/Game/Rumble/Blueprints/GamePlay/BP_SpawnPoint.BP_SpawnPoint_C"))
  (bind _array_element (Utilities|Array|ForEachLoopwithBreak _outactors :!label _label)
    (:LoopBody
      (LocalVariables|SetCurrentSpawnPoint _array_element)
      (if (not (Variables|/Game/Rumble/Blueprints/GamePlay/BP_SpawnPoint.BP_SpawnPoint_C|GetbAlreadyUsed _array_element))
        (Variables|SpawnSystem|SetSpawnPoint (LocalVariables|GetCurrentSpawnPoint))
        (bind _returnvalue (Game|SpawnActorfromClass (Variables|SpawnSystem|GetClassToReSpawn) (Math|Transform|MakeTransform (Transformation|GetWorldLocation (LocalVariables|GetCurrentSpawnPoint)) (Transformation|GetWorldRotation (LocalVariables|GetCurrentSpawnPoint)) "1,1,1") "Undefined" 0 0))
        (Pawn|Possess _returnvalue)
        (Variables|/Game/Rumble/Blueprints/GamePlay/BP_SpawnPoint.BP_SpawnPoint_C|SetbAlreadyUsed (LocalVariables|GetCurrentSpawnPoint) true)
        (goto _label Break)))))

(fn FireatLocation
  (params (SpreadMin :type Float%20%28single-precision%29) (SpreadMax :type Float%20%28single-precision%29))
  (bind _returnvalue (Game|Player|GetPlayerPawn 0))
  (bind _returnvalue_2 (Math|Random|RandomFloatinRange SpreadMin SpreadMax))
  (bind _returnvalue_3 (Transformation|GetActorLocation _returnvalue))
  (bind _returnvalue_4 (Transformation|GetActorRotation _returnvalue))
  (bind _returnvalue_5 (+ (.yaw _returnvalue_4) _returnvalue_2))
  (bind _returnvalue_6 (Math|Rotator|MakeRotator (.roll _returnvalue_4) (.pitch _returnvalue_4) _returnvalue_5))
  (return _returnvalue_6 (+ _returnvalue_3 (* (Math|Vector|GetForwardVector _returnvalue_6) 1e+02)) _returnvalue_3))