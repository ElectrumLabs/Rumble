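; Base GameState for Rumble matches, managing the score-sorted player list, game resets and end-of-game flow, with CheckScore left for DM and TDM children to override.
; Player list changes trigger a descending bubble sort on MyScore, then a multicast scoreboard refresh.
; Multicasts also show or hide the winning screen for a player or team and display the return-to-lobby notice.
; ResetGame respawns players and collectables and zeroes scores.
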(event Custom|MulticastShowWinningScreen
  (params (InPlayerName :type Text))
  ;[1 0 0] Clients and Server | Tells everyone to display the Winning Screen since a player seems to have won
  (Utilities|IsValid (Variables|Default|GetWinningScreenWidgetRef)
    (:Is%20Valid
      _)
    (:Is%20Not%20Valid
      (bind _returnvalue (UserInterface|CreateWidget (Variables|Default|GetWinningScreenClass) (Game|GetPlayerController 0)))
      (bind _output_get (Variables|Default|SetWinningScreenWidgetRef _returnvalue))))
  (UserInterface|Viewport|AddtoViewport _output_get 0)
  (Variables|/Game/Rumble/Widgets/GamePlayBaseWidgets/W_WinningScreenBase.W_WinningScreenBase_C|SetWinningPlayerName (Variables|Default|GetWinningScreenWidgetRef) InPlayerName)
  (Input|SetInputModeUIOnly (Game|GetPlayerController 0) (Variables|Default|GetWinningScreenWidgetRef) "DoNotLock")
  (Variables|/Script/Engine.PlayerController|SetbShowMouseCursor (Game|GetPlayerController 0) true))

(event Custom|MulticastUpdateScoreboard
  (bind _returnvalue (Game|GetPlayerController 0))
  ;[1 0 0] Server | Handles our custom PlayerList
  ;;[1 1 1] Multicast | Tells everyone to update the scoreboard
  (Utilities|IsValid _returnvalue
    (:Is%20Valid
      (bind _asbp_player_controller_base (Utilities|Casting|CastToBP_PlayerController_Base _returnvalue))
      (Default|UpdateScoreboard _asbp_player_controller_base))))

(event Custom|AddPlayerToList
  (params (InPlayerState :type BP%20Player%20State%20Base%20Object%20Reference))
  ;[1 0 0] Server | Handles our custom PlayerList
  ;;[0 0.994 1] Server | Adds the PlayerState to the "MyPlayerList" and sorts it
  (Utilities|Array|Add (Variables|Lists|GetMyPlayerList) InPlayerState)
  (CallFunction|SortPlayerArray))

(event Custom|RemovePlayerFromList
  (params (InPlayerState :type BP%20Player%20State%20Base%20Object%20Reference))
  ;[1 0 0] Server | Handles our custom PlayerList
  ;;[0 1 1] Server | Removes PlayerState from the PlayerList. Also sorts the List
  (Utilities|Array|RemoveItem (Variables|Lists|GetMyPlayerList) InPlayerState)
  (CallFunction|SortPlayerArray)
  (CallFunction|MulticastUpdateScoreboard))

(event Custom|MulticastHideWinningScreen
  (bind _winningscreenwidgetref (Variables|Default|GetWinningScreenWidgetRef))
  ;[1 0 0] Client and Server | Tells everyone to remove the Winning Screen
  (Utilities|IsValid _winningscreenwidgetref
    (:Is%20Valid
      (Widget|RemovefromParent _winningscreenwidgetref)
      (Input|SetInputModeGameOnly (Game|GetPlayerController 0))
      (Variables|/Script/Engine.PlayerController|SetbShowMouseCursor (Game|GetPlayerController 0) false))))

(event Custom|MulticastShowReturnToLobby
  (bind _returnvalue (Game|GetPlayerController 0))
  ;[1 1 1] Remove everybodies ability to move and tell them that the Host is going back to lobby with them
  (Input|DisableInput _returnvalue _returnvalue)
  (bind _returnvalue_2 (UserInterface|CreateWidget "/Game/Rumble/Widgets/GamePlayBaseWidgets/IngameMenuWidgets/W_ReturnToLobby.W_ReturnToLobby_C" (Game|GetPlayerController 0)))
  (UserInterface|Viewport|AddtoViewport _returnvalue_2 0))

(event EventBeginPlay
  ;[1 1 1] Setup Game
  (CallFunction|SetupGame))

(fn ConstructionScript)

(fn CheckScore
  ;[1 1 1] Will be overriden by DM and TDMGamestate
  (return))

(fn ResetPlayerScores
  ;[1 1 1] This will reset the whole Score (even in TeamDeathMatch, because the TeamScore is calculated with the MyScore of each Player) to 0
  (for _array_element (Variables|Default|GetPlayerArray)
    (Utilities|IsValid _array_element
      (:Is%20Valid
        (bind _asbp_player_state_base (Utilities|Casting|CastToBP_PlayerState_Base _array_element))
        (Variables|/Game/Rumble/Blueprints/GamePlay/BP_PlayerState_Base.BP_PlayerState_Base_C|SetMyScore _asbp_player_state_base 0)))))

(fn ResetGame
  ;[1 1 1] Server | We are resetting the Score, the Collectables and respawn all Players! Make sure to destroy Players that are still possessing a Pawn, so we don't duplicate them.
  (bind _outactors (Actor|GetAllActorsOfClass "/Game/Rumble/Blueprints/GamePlay/BP_PlayerController_Base.BP_PlayerController_Base_C"))
  (for _array_element _outactors
    (bind _output_get (LocalVariables|SetCurrentController _array_element))
    (Utilities|IsValid _output_get
      (:Is%20Valid
        (Utilities|IsValid (Pawn|GetControlledPawn (LocalVariables|GetCurrentController)) ; If the Player has a valid pawn, destroy it first and then respawn him
          (:Is%20Valid
            (Actor|DestroyActor (Pawn|GetControlledPawn (LocalVariables|GetCurrentController))))
          (:Is%20Not%20Valid
            _))
        (Default|RespawnPlayer (LocalVariables|GetCurrentController)))))
  (CallFunction|ResetPlayerScores)
  (CallFunction|ResetCollectables)
  (CallFunction|MulticastHideWinningScreen))

(fn FinishGame
  (params (InPlayerState :type BP%20Player%20State%20Base%20Object%20Reference) (InWinningName :type Text))
  ;[1 1 1] Server | When finishing the game, we tell everyone to show our Winning Screen Widget and providing the Name of the winning player. If the Player is not valid, we have a Team that won the Game, so we provide the Teamname
  (Utilities|IsValid InPlayerState
    (:Is%20Valid
      (CallFunction|MulticastShowWinningScreen (Utilities|Text|ToText(String) (Variables|/Script/Engine.PlayerState|GetPlayerName InPlayerState))))
    (:Is%20Not%20Valid
      (CallFunction|MulticastShowWinningScreen InWinningName))))

(fn ResetCollectables
  ;[1 1 1] Respawns all collectables if needed
  (bind _outactors (Actor|GetAllActorsOfClass "/Game/Rumble/Blueprints/GamePlay/BP_Platform_Base.BP_Platform_Base_C"))
  (for _array_element _outactors
    (Utilities|IsValid _array_element
      (:Is%20Valid
        (Default|RespawnCollectable _array_element)))))

(fn SortPlayerArray
  ;[1 1 1] We use a very basic sort algorithm for our Arrays. It is called "Bubblesort". Best thing would be looking it up with google, because it is better explained on the internet. I used the second algorithm on the Wikipedia page. TL;DR: we check a pair of Scores that are directly behind each other and swap them if the first one is less than the second one
  (LocalVariables|SetCurrentLoopEnd (Utilities|Array|Length (Variables|Lists|GetMyPlayerList)))
  (bind _output_get (LocalVariables|SetbDoOnce true))
  (while (or _output_get (LocalVariables|GetbSwapped))
    (LocalVariables|SetbDoOnce false)
    (LocalVariables|SetbSwapped false)
    (for _index (range 0 (- (LocalVariables|GetCurrentLoopEnd) 2))
      (LocalVariables|Set_CurrentIndex1 _index)
      (LocalVariables|Set_CurrentIndex2 (+ (LocalVariables|Get_CurrentIndex1) 1))
      (if (>= (Variables|/Game/Rumble/Blueprints/GamePlay/BP_PlayerState_Base.BP_PlayerState_Base_C|GetMyScore (Utilities|Array|Get(acopy) (Variables|Lists|GetMyPlayerList) (LocalVariables|Get_CurrentIndex2))) (Variables|/Game/Rumble/Blueprints/GamePlay/BP_PlayerState_Base.BP_PlayerState_Base_C|GetMyScore (Utilities|Array|Get(acopy) (Variables|Lists|GetMyPlayerList) (LocalVariables|Get_CurrentIndex1))))
        (CallFunction|SwapArrayElements (LocalVariables|Get_CurrentIndex1) (LocalVariables|Get_CurrentIndex2))
        (LocalVariables|SetbSwapped true)))
    (LocalVariables|SetCurrentLoopEnd (- (LocalVariables|GetCurrentLoopEnd) 1)))
  (CallFunction|MulticastUpdateScoreboard))

(fn SwapArrayElements
  (params (InIndex1 :type Integer) (InIndex2 :type Integer))
  ;[1 1 1] We save the first Element in TempPS, override the first Element with the second one and set the second one to the Temp one.
  (LocalVariables|Set_Index1 InIndex1)
  (LocalVariables|Set_Index2 InIndex2)
  (LocalVariables|SetTempPS (Utilities|Array|Get(acopy) (Variables|Lists|GetMyPlayerList) (LocalVariables|Get_Index1)))
  (Utilities|Array|SetArrayElem (Variables|Lists|GetMyPlayerList) (LocalVariables|Get_Index1) (Utilities|Array|Get(acopy) (Variables|Lists|GetMyPlayerList) (LocalVariables|Get_Index2)))
  (Utilities|Array|SetArrayElem (Variables|Lists|GetMyPlayerList) (LocalVariables|Get_Index2) (LocalVariables|GetTempPS)))

(fn SetupGame
  (bind _returnvalue (Game|GetGameInstance))
  ;[1 1 1] Give focus to the Game
  (Class|WidgetBlueprintLibrary|SetFocustoGameViewport)
  (Input|SetInputModeGameOnly (Game|GetPlayerController 0))
  ;[1 1 1] Tell GameInstance to Transition to Playing State
  (Utilities|IsValid _returnvalue
    (:Is%20Valid
      (bind _asbp_game_instance (Utilities|Casting|CastToBP_GameInstance _returnvalue))
      (Default|TransitiontoState _asbp_game_instance "NewEnumerator2"))))