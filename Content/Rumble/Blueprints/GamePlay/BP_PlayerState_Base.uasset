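; Base PlayerState for Rumble that sets the player's name, registers the player with the game state and tracks a score.
; BeginPlay caches game instance, controller and game state references, then applies the saved name through a SetName console command, going via a server event on remote machines.
; On authority it joins the GameState player list, skipping ownerless dummies, and leaves on EndPlay.
; AddScore increments the score, then has the GameState sort players and check the score.
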(event Custom|ServerSetPlayerName
  (params (InPlayerName :type Text))
  ;[1 1 1] Takes care of setting the PlayerName via ConsoleCommand
  (CallFunction|SetPlayerName InPlayerName))

(event Custom|SetPlayerName
  (params (InPlayerName :type Text))
  ;[1 1 1] Takes care of setting the PlayerName via ConsoleCommand
  (Utilities|IsValid (Variables|Default|GetOwningPlayerControllerRef)
    (:Is%20Valid
      (Development|ExecuteConsoleCommand (Utilities|String|Append "SetName " (Utilities|String|ToString(Text) InPlayerName)) (Variables|Default|GetOwningPlayerControllerRef)))))

(event Custom|SetupReferences
  (bind _returnvalue (Components|GetOwner))
  (bind _returnvalue_2 (Game|GetGameState))
  (bind _returnvalue_3 (Game|GetGameInstance))
  ;[1 1 1] Setup important reference so we don't need to cast them all the time
  (Utilities|FlowControl|Sequence
    (:then_0
      (Utilities|IsValid _returnvalue_3
        (:Is%20Valid
          (bind _asbp_game_instance (Utilities|Casting|CastToBP_GameInstance _returnvalue_3))
          (Variables|Default|SetGameInstanceRef _asbp_game_instance))))
    (:then_1
      (Utilities|IsValid _returnvalue
        (:Is%20Valid
          (bind _asbp_player_controller_base (Utilities|Casting|CastToBP_PlayerController_Base _returnvalue))
          (Variables|Default|SetOwningPlayerControllerRef _asbp_player_controller_base))))
    (:then_2
      (Utilities|IsValid _returnvalue_2
        (:Is%20Valid
          (bind _asbp_game_state_base (Utilities|Casting|CastToBP_GameState_Base _returnvalue_2))
          (Variables|Default|SetGameStateRef _asbp_game_state_base))))))

(event Custom|AddScore
  ;[1 1 1] Adds 1 to the score, sorts the Player Arrays and checks if someone won
  (Math|Integer|IncrementInt (Variables|CharacterProperties|GetMyScore)
    (:%20%20
      (Utilities|IsValid (Variables|Default|GetGameStateRef)
        (:Is%20Valid
          (Default|SortPlayerArray (Variables|Default|GetGameStateRef))
          (Default|CheckScore (Variables|Default|GetGameStateRef)))))))

(event EventEndPlay
  (params (EndPlayReason :type EEndPlayReason%20Enum :default "Destroyed"))
  (bind _gamestateref (Variables|Default|GetGameStateRef))
  ;[1 0 0] When the Game ends, we remove the PlayerState from the List
  (Networking|SwitchHasAuthority
    (:Authority
      (Utilities|IsValid _gamestateref
        (:Is%20Valid
          (Default|RemovePlayerfromList _gamestateref self))))))

(event EventBeginPlay
  (bind _gameinstanceref (Variables|Default|GetGameInstanceRef))
  (bind _gamestateref (Variables|Default|GetGameStateRef))
  (bind _tempgameusersettings (Variables|/Game/Rumble/Blueprints/BlueprintsUsedInAllMaps/BP_GameInstance.BP_GameInstance_C|GetTempGameUserSettings _gameinstanceref))
  (bind _playername (Utilities|Struct|BreakFGameUserSettings _tempgameusersettings))
  ;[0 0 0] Server and Clients | Sets our PlayerName at the beginning and sets the Health and Mana to a random Number, so that we have some different values to show
  (CallFunction|SetupReferences)
  (Utilities|FlowControl|Sequence
    (:then_0
      (Utilities|IsValid _gameinstanceref
        (:Is%20Valid
          (Networking|SwitchHasAuthority
            (:Authority
              (CallFunction|SetPlayerName _playername))
            (:Remote
              (CallFunction|ServerSetPlayername _playername))))))
    (:then_1
      (Networking|SwitchHasAuthority
        (:Authority
          (Utilities|IsValid (Components|GetOwner) ; Prevents Dummy PlayerState from being added
            (:Is%20Valid
              (Utilities|IsValid _gamestateref
                (:Is%20Valid
                  (Default|AddPlayertoList _gamestateref self))))))))))

(fn ConstructionScript)