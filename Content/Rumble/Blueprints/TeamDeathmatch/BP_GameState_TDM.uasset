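; Team Deathmatch GameState that tracks Red and Blue team rosters and their combined scores.
; AddToTeam places each PlayerState into a team array based on its red-team flag.
; On the server, Tick recomputes both totals every frame by summing each valid member's score into the team score variables.
; CheckScore compares those totals to the winning score and finishes the game naming the winning team, with Red checked first.
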(event Custom|AddToTeam
  (params (InPlayerState :type BP%20Player%20State%20TDM%20Object%20Reference))
  ;[1 1 0] Server | Adds the Calling PlayerState to one of the Lists, based on the "bIsRedTeam" Bool
  (if (Variables|/Game/Rumble/Blueprints/TeamDeathmatch/BP_PlayerState_TDM.BP_PlayerState_TDM_C|GetbIsRedTeam InPlayerState)
    (Utilities|Array|AddUnique (Variables|Lists|GetRedTeam) InPlayerState)
    (else
      (Utilities|Array|AddUnique (Variables|Lists|GetBlueTeam) InPlayerState))))

(event EventTick
  (params (DeltaSeconds :type Float%20%28single-precision%29))
  ;[0 1 1] Server | Calculating the overall Team Scores and saving it to the Score Variables
  (Networking|SwitchHasAuthority
    (:Authority
      (bind (_outredteamscore _outblueteamscore) (CallFunction|CalculateTeamScore))
      (Variables|ScoreSystem|SetRedTeamScore _outredteamscore)
      (Variables|ScoreSystem|SetBlueTeamScore _outblueteamscore))))

(fn ConstructionScript)

(fn CheckScore
  ;[1 1 1] Checks if either the Red or the Blue Team got the minimum Score to win
  (bind (_outredteamscore _outblueteamscore) (CallFunction|CalculateTeamScore))
  (LocalVariables|SetbRedTeamWon (>= _outredteamscore (Variables|ScoreSystem|GetWinningScore)))
  (LocalVariables|SetbBlueTeamWon (>= _outblueteamscore (Variables|ScoreSystem|GetWinningScore)))
  (if (LocalVariables|GetbRedTeamWon)
    (CallFunction|FinishGame 0 "Red Team")
    (elif (LocalVariables|GetbBlueTeamWon)
      (CallFunction|FinishGame 0 "Blue Team"))))

(fn CalculateTeamScore
  ;[0 1 1] Server | Calculating the overall Team Scores by getting the Team Arrays and using the PlayerStates inside of them
  (Networking|SwitchHasAuthority
    (:Authority
      (Utilities|FlowControl|Sequence
        (:then_0
          (LocalVariables|SetReturnRedScore 0)
          (for _array_element (Variables|Lists|GetRedTeam)
            (Utilities|IsValid _array_element
              (:Is%20Valid
                (LocalVariables|SetReturnRedScore (+ (Variables|/Game/Rumble/Blueprints/GamePlay/BP_PlayerState_Base.BP_PlayerState_Base_C|GetMyScore _array_element) (LocalVariables|GetReturnRedScore)))))))
        (:then_1
          (LocalVariables|SetReturnBlueScore 0)
          (for _array_element_2 (Variables|Lists|GetBlueTeam)
            (Utilities|IsValid _array_element_2
              (:Is%20Valid
                (LocalVariables|SetReturnBlueScore (+ (Variables|/Game/Rumble/Blueprints/GamePlay/BP_PlayerState_Base.BP_PlayerState_Base_C|GetMyScore _array_element_2) (LocalVariables|GetReturnBlueScore)))))))
        (:then_2
          (return (LocalVariables|GetReturnRedScore) (LocalVariables|GetReturnBlueScore)))))
    (:Remote
      (return 0 0))))