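; Deathmatch game state that overrides the base class's server-side score check to end the match once a player reaches the winning score.
; CheckScore loops over PlayerArray, casts entries to BP_PlayerState_Base and flags a win when MyScore meets WinningScore.
; PlayerStateRef updates on every cast player, so FinishGame receives the last one iterated, which may differ from the player who reached the threshold.
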(fn ConstructionScript
  (|CallParentFunction))

(fn CheckScore
  ;[1 1 1] Server | Check if someone reached the minimum score to win the game. This function is overriden from the GameStateBase class which is the Parent class of this GameState
  (for _array_element (Variables|Default|GetPlayerArray)
    (Utilities|IsValid _array_element
      (:Is%20Valid
        (bind _asbp_player_state_base (Utilities|Casting|CastToBP_PlayerState_Base _array_element))
        (LocalVariables|SetPlayerStateRef _asbp_player_state_base)
        (if (>= (Variables|/Game/Rumble/Blueprints/GamePlay/BP_PlayerState_Base.BP_PlayerState_Base_C|GetMyScore _asbp_player_state_base) (Variables|Default|GetWinningScore))
          (LocalVariables|SetbSomeOneWon true)))))
  (if (LocalVariables|GetbSomeOneWon)
    (CallFunction|FinishGame (LocalVariables|GetPlayerStateRef))))