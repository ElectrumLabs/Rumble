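; Lobby GameState that tracks players, red and blue teams and selected character classes for the multiplayer lobby.
; On the server it copies the GameMode's rules for display on clients and spawns a shared replicated model viewer.
; Joining players alternate between teams via FlipFlop in team games and can switch sides.
; Player and team arrays are reassigned after edits to fire OnReps that refresh the lobby widget through the GameInstance.
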(event Custom|SetupModelViewers
  ;[1 1 1] Spawn the Model Viewer replicated, so everyone can use it in their Lobby UI
  (Networking|SwitchHasAuthority
    (:Authority
      (bind _returnvalue (Game|SpawnActorfromClass "/Game/Rumble/Blueprints/Lobby/BP_ModelViewer.BP_ModelViewer_C" (Math|Transform|MakeTransform "0, 0,1000.000000" "0, 0, 0" "1,1,1") "AlwaysSpawn" 0 0))
      (Variables|References|SetModelViewerRef _returnvalue))))

(event Custom|AddPlayerToLists
  (params (InPlayerState :type BP%20Player%20State%20Lobby%20Object%20Reference))
  ;[1 0 0] Server | Overall List Logic. These functions are called from ServerSide within the PlayerState Class
  ;;[1 0 1] Server | Adds a new Player to the "CharacterPlayerList" and also to one of the "TeamList"s if we are in a TDM Game
  (Utilities|IsValid InPlayerState
    (:Is%20Valid
      (CallFunction|AddtoCharacterPlayerList InPlayerState)
      (if (Variables|SettingsandRules|GetbIsTeamGame)
        (CallFunction|AddPlayertoTeam InPlayerState)
        (else
          (CallFunction|MulticastUpdatePlayerList))))))

(event Custom|SetupReferences
  (bind _returnvalue (Game|GetPlayerController 0))
  (bind _returnvalue_2 (Game|GetGameInstance))
  (bind _authoritygamemode (Variables|Default|GetAuthorityGameMode))
  ;[1 1 1] Setup all references, so we don't need to cast every time
  (Utilities|FlowControl|Sequence
    (:then_0
      (Utilities|IsValid _returnvalue_2
        (:Is%20Valid
          (bind _asbp_game_instance (Utilities|Casting|CastToBP_GameInstance _returnvalue_2))
          (Variables|References|SetGameInstanceRef _asbp_game_instance))))
    (:then_1
      (Utilities|IsValid _returnvalue
        (:Is%20Valid
          (bind _asbp_player_controller_lobby (Utilities|Casting|CastToBP_PlayerController_Lobby _returnvalue))
          (Variables|References|SetPlayerControllerRef _asbp_player_controller_lobby))))
    (:then_2
      (Utilities|IsValid _authoritygamemode
        (:Is%20Valid
          (bind _asbp_game_mode_lobby (Utilities|Casting|CastToBP_GameMode_Lobby _authoritygamemode))
          (Variables|References|SetGameModeRef _asbp_game_mode_lobby))))))

(event Custom|AddPlayerToBlueTeam
  (params (InPlayerState :type BP%20Player%20State%20Lobby%20Object%20Reference))
  ;[1 0 0] Server | "TeamList" logic. These functions are called from server side
  ;;[0 1 1] Server | Adds a new Player to one of the Teams. Also sets the "bIsRedPlayer" bool, which calls a RepNotify function "OnRep_bIsRedPlayer" inside of the "LobbyPlayerState"
  (Utilities|Array|AddUnique (Variables|Lists|GetBlueTeam) InPlayerState)
  (Variables|/Game/Rumble/Blueprints/Lobby/BP_PlayerState_Lobby.BP_PlayerState_Lobby_C|SetbIsRedPlayer InPlayerState false)
  (Variables|Lists|SetBlueTeam (Variables|Lists|GetBlueTeam)))

(event Custom|AddPlayerToRedTeam
  (params (InPlayerState :type BP%20Player%20State%20Lobby%20Object%20Reference))
  ;[1 0 0] Server | "TeamList" logic. These functions are called from server side
  ;;[0 1 1] Server | Adds a new Player to one of the Teams. Also sets the "bIsRedPlayer" bool, which calls a RepNotify function "OnRep_bIsRedPlayer" inside of the "LobbyPlayerState"
  (Utilities|Array|AddUnique (Variables|Lists|GetRedTeam) InPlayerState)
  (Variables|/Game/Rumble/Blueprints/Lobby/BP_PlayerState_Lobby.BP_PlayerState_Lobby_C|SetbIsRedPlayer InPlayerState true)
  (Variables|Lists|SetRedTeam (Variables|Lists|GetRedTeam)))

(event Custom|AddPlayerToTeam
  (params (InPlayerState :type BP%20Player%20State%20Lobby%20Object%20Reference))
  ;[1 0 0] Server | "TeamList" logic. These functions are called from server side
  ;;[0 1 1] Server | Adds a Player to Blue/Red team after one another
  (Utilities|FlowControl|FlipFlop
    (:A
      (CallFunction|AddPlayertoRedTeam InPlayerState))
    (:B
      (CallFunction|AddPlayertoBlueTeam InPlayerState))))

(event Custom|RemovePlayerFromTeamList
  (params (InPlayerState :type BP%20Player%20State%20Lobby%20Object%20Reference))
  ;[1 0 0] Server | "TeamList" logic. These functions are called from server side
  ;;[0 1 1] Server | Removes the Player from from the red or the blue team, based on the team he is on. This is saved in the "bIsRedTeam" bool of the "LobbyPlayerState"
  (Utilities|IsValid InPlayerState
    (:Is%20Valid
      (if (Variables|/Game/Rumble/Blueprints/Lobby/BP_PlayerState_Lobby.BP_PlayerState_Lobby_C|GetbIsRedPlayer InPlayerState)
        (Utilities|Array|RemoveItem (Variables|Lists|GetRedTeam) InPlayerState)
        (Variables|Lists|SetRedTeam (Variables|Lists|GetRedTeam))
        (else
          (Utilities|Array|RemoveItem (Variables|Lists|GetBlueTeam) InPlayerState)
          (Variables|Lists|SetBlueTeam (Variables|Lists|GetBlueTeam)))))))

(event Custom|GetGameModeRules
  (bind _gamemoderef (Variables|References|GetGameModeRef))
  ;[1 0 0] Server | Inits several things on BeginPlay ServerSide. Follow the Functions and the comments
  ;;[0 0 0] Server | Get all Rules from the GameMode, so we can display them replicated on Clients
  (Networking|SwitchHasAuthority
    (:Authority
      (Utilities|IsValid _gamemoderef
        (:Is%20Valid
          (Variables|SettingsandRules|SetbIsTeamGame (Variables|/Game/Rumble/Blueprints/Lobby/BP_GameMode_Lobby.BP_GameMode_Lobby_C|GetbIsTeamGame _gamemoderef))
          (Variables|SettingsAndRules|SetServerName (Utilities|Text|ToText(String) (Variables|/Game/Rumble/Blueprints/Lobby/BP_GameMode_Lobby.BP_GameMode_Lobby_C|GetServerName _gamemoderef)))
          (Variables|SettingsandRules|SetMaxNumPlayers (Variables|/Game/Rumble/Blueprints/Lobby/BP_GameMode_Lobby.BP_GameMode_Lobby_C|GetMaxNumPlayers _gamemoderef))
          (Variables|SettingsandRules|SetSelectedGameMode (Utilities|Text|ToText(String) (Variables|/Game/Rumble/Blueprints/Lobby/BP_GameMode_Lobby.BP_GameMode_Lobby_C|GetSelectedGameMode _gamemoderef)))
          (Variables|SettingsAndRules|SetCharacterClasses (Variables|/Game/Rumble/Blueprints/Lobby/BP_GameMode_Lobby.BP_GameMode_Lobby_C|GetPlayerClasses _gamemoderef))
          (Variables|SettingsAndRules|SetbOnlyUniqueSelection (Variables|/Game/Rumble/Blueprints/Lobby/BP_GameMode_Lobby.BP_GameMode_Lobby_C|GetbOnlyUniqueSelection _gamemoderef))
          (Variables|SettingsAndRules|SetSelectedGamePlayMap (Utilities|Text|ToText(String) (Variables|/Game/Rumble/Blueprints/Lobby/BP_GameMode_Lobby.BP_GameMode_Lobby_C|GetSelectedGamePlayMap _gamemoderef))))))))

(event Custom|SwitchTeam
  (params (InPlayerState :type BP%20Player%20State%20Lobby%20Object%20Reference))
  ;[1 0 0] Server | "TeamList" logic. These functions are called from server side
  ;;[0 1 1] Server | Switches the Player to the other Team, base on the "bIsRedPlayer" bool of the "LobbyPlayerState"
  (Utilities|IsValid InPlayerState
    (:Is%20Valid
      (CallFunction|RemovePlayerfromTeamList InPlayerState)
      (if (Variables|/Game/Rumble/Blueprints/Lobby/BP_PlayerState_Lobby.BP_PlayerState_Lobby_C|GetbIsRedPlayer InPlayerState)
        (CallFunction|AddPlayertoBlueTeam InPlayerState)
        (else
          (CallFunction|AddPlayertoRedTeam InPlayerState))))))

(event Custom|MulticastUpdatePlayerList
  (bind _gameinstanceref (Variables|References|GetGameInstanceRef))
  (bind _lobbywidgetref (Variables|/Game/Rumble/Blueprints/BlueprintsUsedInAllMaps/BP_GameInstance.BP_GameInstance_C|GetLobbyWidgetRef _gameinstanceref))
  ;[1 1 1] Tell everyone to update the PlayerList
  (Utilities|IsValid _gameinstanceref
    (:Is%20Valid
      (Utilities|IsValid _lobbywidgetref
        (:Is%20Valid
          (Default|UpdatePlayerList _lobbywidgetref))))))

(event Custom|RemovePlayerFromLists
  (params (InPlayerState :type BP%20Player%20State%20Lobby%20Object%20Reference))
  ;[1 0 0] Server | Overall List Logic. These functions are called from ServerSide within the PlayerState Class
  ;;[1 0 1] Server | Removes a Player from the "CharacterPlayerList" and also from the "TeamList"s if we are in a TDM Game
  (Utilities|IsValid InPlayerState
    (:Is%20Valid
      (CallFunction|RemovefromCharacterPlayerList InPlayerState)
      (if (Variables|SettingsandRules|GetbIsTeamGame)
        (CallFunction|RemovePlayerfromTeamList InPlayerState)
        (else
          (CallFunction|MulticastUpdatePlayerList))))))

(event EventBeginPlay
  ;[1 0 0] Server | Inits several things on BeginPlay ServerSide. Follow the Functions and the comments
  ;;[0 0 0] Server | Inits the "CharacterPlayerList" and gets the GameMode Rules
  (CallFunction|SetupReferences)
  (CallFunction|GetGameModeRules)
  (CallFunction|SetupModelViewers))

(fn ConstructionScript)

(fn OnRepBlueTeam
  (bind _gameinstanceref (Variables|References|GetGameInstanceRef))
  (bind _lobbywidgetref (Variables|/Game/Rumble/Blueprints/BlueprintsUsedInAllMaps/BP_GameInstance.BP_GameInstance_C|GetLobbyWidgetRef _gameinstanceref))
  ;[1 1 1] When the CharacterPlayer List updates, tell everyone to update their Widgets
  (Utilities|IsValid _gameinstanceref
    (:Is%20Valid
      (Utilities|IsValid _lobbywidgetref
        (:Is%20Valid
          (Default|UpdateTeamList _lobbywidgetref))))))

(fn OnRepRedTeam
  (bind _gameinstanceref (Variables|References|GetGameInstanceRef))
  (bind _lobbywidgetref (Variables|/Game/Rumble/Blueprints/BlueprintsUsedInAllMaps/BP_GameInstance.BP_GameInstance_C|GetLobbyWidgetRef _gameinstanceref))
  ;[1 1 1] When the CharacterPlayer List updates, tell everyone to update their Widgets
  (Utilities|IsValid _gameinstanceref
    (:Is%20Valid
      (Utilities|IsValid _lobbywidgetref
        (:Is%20Valid
          (Default|UpdateTeamList _lobbywidgetref))))))

(fn AddtoCharacterPlayerList
  (params (InPlayerState :type BP%20Player%20State%20Lobby%20Object%20Reference))
  (LocalVariables|SetNewPlayer InPlayerState)
  (Utilities|Array|Add (Variables|Lists|GetCharacterPlayerList) (LocalVariables|GetNewPlayer))
  (Variables|Lists|SetCharacterPlayerList (Variables|Lists|GetCharacterPlayerList)) ; We need to set the Array again, so the "OnRep" function will be called...
)

(fn RemovefromCharacterPlayerList
  (params (InPlayerState :type BP%20Player%20State%20Lobby%20Object%20Reference))
  ;[1 1 1] Remove the Saved Selected Character and the Player itself. Also set the Array so the OnRep gets called
  (LocalVariables|SetPlayerToRemove InPlayerState)
  (if (Utilities|Array|IsValidIndex (Variables|Lists|GetCharacterPlayerList) (Utilities|Array|FindItem (Variables|Lists|GetCharacterPlayerList) (LocalVariables|GetPlayerToRemove)))
    (Utilities|Array|RemoveIndex (Variables|Lists|GetSelectedCharacterClasses) (Utilities|Array|FindItem (Variables|Lists|GetCharacterPlayerList) (LocalVariables|GetPlayerToRemove)))
    (Utilities|Array|RemoveItem (Variables|Lists|GetCharacterPlayerList) (LocalVariables|GetPlayerToRemove))
    (Variables|Lists|SetCharacterPlayerList (Variables|Lists|GetCharacterPlayerList))))

(fn OnRepCharacterPlayerList
  (bind _gameinstanceref (Variables|References|GetGameInstanceRef))
  (bind _lobbywidgetref (Variables|/Game/Rumble/Blueprints/BlueprintsUsedInAllMaps/BP_GameInstance.BP_GameInstance_C|GetLobbyWidgetRef _gameinstanceref))
  ;[1 1 1] When the CharacterPlayer List updates, tell everyone to update their Widgets
  (Utilities|IsValid _gameinstanceref
    (:Is%20Valid
      (Utilities|IsValid _lobbywidgetref
        (:Is%20Valid
          (Default|UpdateCharacterList _lobbywidgetref))))))

(fn CheckifCharacterClassAlreadyTaken
  (params (InNewClass :type F%20Select%20Class%20Structure) (InOldClass :type F%20Select%20Class%20Structure))
  (LocalVariables|SetNewClass InNewClass)
  (CallFunction|RemoveSelectedClass InOldClass)
  (for _array_element (Variables|Lists|GetSelectedCharacterClasses)
    (if (== (.class _array_element) (.class (LocalVariables|GetNewClass)))
      (LocalVariables|SetbAlreadyTaken true)))
  (return (LocalVariables|GetbAlreadyTaken)))

(fn IsTeamGame
  (return (Variables|SettingsandRules|GetbIsTeamGame)))

(fn UniqueSelectionActive
  (return (Variables|SettingsAndRules|GetbOnlyUniqueSelection)))

(fn RemoveSelectedClass
  (params (InClass :type F%20Select%20Class%20Structure))
  (Utilities|Array|RemoveItem (Variables|Lists|GetSelectedCharacterClasses) InClass))

(fn AddSelectedClass
  (params (InClass :type F%20Select%20Class%20Structure))
  (Utilities|Array|Add (Variables|Lists|GetSelectedCharacterClasses) InClass))