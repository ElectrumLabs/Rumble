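; Lobby PlayerState that holds each player's name, ready state, team and selected character class.
; On BeginPlay it caches references, sets the GameInstance's saved name server-side via a SetName console command, and registers with the lobby GameState, unregistering on EndPlay.
; Ready toggles apply on the client first, then on the server.
; The server validates class picks against optional unique selection; class and team are copied to the local GameInstance.
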(event Custom|ServerSetSelectedClass
  (params (InClass :type F%20Select%20Class%20Structure))
  (bind _gamestateref (Variables|Default|GetGameStateRef))
  ;[0 0 0] Server | Sets SelectedClass. Called from Widget (Client Side). Executes on Server
  (Utilities|IsValid _gamestateref
    (:Is%20Valid
      (bind _return_value (Default|UniqueSelectionActive _gamestateref))
      (if _return_value
        (bind _boutistaken (Default|CheckifCharacterClassAlreadyTaken _gamestateref InClass (Variables|Default|GetSelectedClass)))
        (if _boutistaken
          (Variables|Default|SetSelectedClass "")
          (else
            (bind _output_get (Variables|Default|SetSelectedClass InClass))
            (Default|AddSelectedClass (Variables|Default|GetGameStateRef) _output_get)))
        (else
          (Variables|Default|SetSelectedClass InClass)))
      (CallFunction|ClientSaveSelectClass (Variables|Default|GetSelectedClass)))))

(event Custom|ServerSetPlayerName
  (params (InPlayerName :type Text))
  ;[0 0 0] Server | Sets the PlayerName. Asked by Client. Executed on Server
  (CallFunction|SetPlayerName InPlayerName))

(event Custom|SetupReferences
  (bind _returnvalue (Components|GetOwner))
  (bind _returnvalue_2 (Game|GetGameState))
  (bind _returnvalue_3 (Game|GetGameInstance))
  ;[1 1 1] Get all kinds of important references so we don't need to cast all the time
  (Utilities|FlowControl|Sequence
    (:then_0
      (Utilities|IsValid _returnvalue_3
        (:Is%20Valid
          (bind _asbp_game_instance (Utilities|Casting|CastToBP_GameInstance _returnvalue_3))
          (Variables|Default|SetGameInstanceRef _asbp_game_instance))))
    (:then_1
      (Utilities|IsValid _returnvalue
        (:Is%20Valid
          (bind _asbp_player_controller_lobby (Utilities|Casting|CastToBP_PlayerController_Lobby _returnvalue))
          (Variables|Default|SetOwningPlayerControllerRef _asbp_player_controller_lobby))))
    (:then_2
      (Utilities|IsValid _returnvalue_2
        (:Is%20Valid
          (bind _asbp_game_state_lobby (Utilities|Casting|CastToBP_GameState_Lobby _returnvalue_2))
          (Variables|Default|SetGameStateRef _asbp_game_state_lobby))))))

(event Custom|SetPlayerName
  (params (InPlayerName :type Text))
  ;[1 1 1] Set Owning Players Name with Console Command as GameMode function crashs
  (Utilities|IsValid (Variables|Default|GetOwningPlayerControllerRef)
    (:Is%20Valid
      (Development|ExecuteConsoleCommand (Utilities|String|Append "SetName " (Utilities|String|ToString(Text) InPlayerName)) (Variables|Default|GetOwningPlayerControllerRef)))))

(event Custom|ToggleIsReady
  ;[0 0 0] Let's the Client set it's own Ready State before replication to avoid lag
  (Variables|Default|SetbIsReady (not (Variables|Default|GetbIsReady)))
  (Networking|SwitchHasAuthority
    (:Remote
      (CallFunction|ServerToggleIsReady))))

(event Custom|ServerToggleIsReady
  ;[0 0 0] Server | Sets Ready State
  (Variables|Default|SetbIsReady (not (Variables|Default|GetbIsReady))))

(event Custom|ClientSaveSelectClass
  (params (InClass :type F%20Select%20Class%20Structure))
  (bind _returnvalue (Game|GetGameInstance))
  ;[0 0 0] Tell the Client to save its selected class
  (Utilities|IsValid _returnvalue
    (:Is%20Valid
      (bind _asbp_game_instance (Utilities|Casting|CastToBP_GameInstance _returnvalue))
      (Variables|/Game/Rumble/Blueprints/BlueprintsUsedInAllMaps/BP_GameInstance.BP_GameInstance_C|SetSelectedCharacterClass _asbp_game_instance InClass))))

(event EventEndPlay
  (params (EndPlayReason :type EEndPlayReason%20Enum :default "Destroyed"))
  (bind _gamestateref (Variables|Default|GetGameStateRef))
  ;[0 1 0] Server | When this actor gets removed from the Game, the Server Version will call the GameState function to remove the PlayerState from all lists and make sure the selected character gets reseted
  (Networking|SwitchHasAuthority
    (:Authority
      (Utilities|IsValid _gamestateref
        (:Is%20Valid
          (Default|RemovePlayerfromLists _gamestateref self))))))

(event EventBeginPlay
  (bind _gameinstanceref (Variables|Default|GetGameInstanceRef))
  (bind _gamestateref (Variables|Default|GetGameStateRef))
  (bind _tempgameusersettings (Variables|/Game/Rumble/Blueprints/BlueprintsUsedInAllMaps/BP_GameInstance.BP_GameInstance_C|GetTempGameUserSettings _gameinstanceref))
  (bind _playername (Utilities|Struct|BreakFGameUserSettings _tempgameusersettings))
  ;[1 0 1] When the PlayerState calls BeginPlay, we get the PlayerName from our GameInstance and let the Server set the replicated variable, so everyone can see it. Also tell the GameState to add the Player(State) to the PlayerState Lists of the GameState
  (Utilities|IsValid (Components|GetOwner) ; Prevents Dummy PlayerState from being added
    (:Is%20Valid
      (CallFunction|SetupReferences)
      (Utilities|FlowControl|Sequence
        (:then_0
          (Utilities|IsValid _gameinstanceref
            (:Is%20Valid
              (Networking|SwitchHasAuthority
                (:Authority
                  (CallFunction|SetPlayerName _playername))
                (:Remote
                  (CallFunction|ServerSetPlayername _playername))))))
        (:then_1
          (Networking|SwitchHasAuthority
            (:Authority
              (Utilities|IsValid _gamestateref
                (:Is%20Valid
                  (Default|AddPlayertoLists _gamestateref self))))))))
    (:Is%20Not%20Valid
      (Actor|DestroyActor))))

(fn ConstructionScript)

(fn OnRepBIsRedPlayer
  (bind _returnvalue (Components|GetOwner))
  (bind _gameinstanceref (Variables|Default|GetGameInstanceRef))
  ;[1 1 1] RepNotify | Everytime the Replicated Variable gets updated by the server, this function gets called and updates the GameInstance version of that variable for the controlling client
  (Utilities|IsValid _returnvalue
    (:Is%20Valid
      (bind _asplayer_controller (Utilities|Casting|CastToPlayerController _returnvalue))
      (if (Pawn|IsLocalPlayerController _asplayer_controller)
        (Utilities|IsValid _gameinstanceref
          (:Is%20Valid
            (Variables|/Game/Rumble/Blueprints/BlueprintsUsedInAllMaps/BP_GameInstance.BP_GameInstance_C|SetbIsRedTeam _gameinstanceref (Variables|Default|GetbIsRedPlayer))))))))